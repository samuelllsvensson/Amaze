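; Bookshelf actor that swings open like a door when its OpenDoor event is called.
; A DoOnce gate limits the opening to a single time, playing a creaking sound at the actor's location and storing the starting rotation.
; A timeline then adds a vector track to that stored rotation each update, rotating the whole actor relative to its initial orientation.
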(event `OpenDoor`
  (`/Engine/EditorBlueprintResources/StandardMacros.DoOnce` false
    (:`Completed`
      (`GameplayStatics.PlaySoundAtLocation` "/Game/Sounds/CreakingDoor.CreakingDoor" (`self.K2_GetActorLocation`))
      (set `self.start_rot` (`self.K2_GetActorRotation`))
      (bind (_direction _newtrack_0) (`Timeline|Timeline_0`)
        (:`Update`
          (`self.K2_SetActorRotation` (`KismetMathLibrary.MakeRotator` (.x (+ _newtrack_0 (`KismetMathLibrary.MakeVector` (.roll (`self.start_rot`)) (.pitch (`self.start_rot`)) (.yaw (`self.start_rot`))))) (.y (+ _newtrack_0 (`KismetMathLibrary.MakeVector` (.roll (`self.start_rot`)) (.pitch (`self.start_rot`)) (.yaw (`self.start_rot`))))) (.z (+ _newtrack_0 (`KismetMathLibrary.MakeVector` (.roll (`self.start_rot`)) (.pitch (`self.start_rot`)) (.yaw (`self.start_rot`))))))))))))

(fn `UserConstructionScript`)